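; Placeable actor that teleports the player's BP_My_Character when T is pressed.
; On BeginPlay it enables input from player controller 0 and makes that controller its owner.
; T moves the character to PlayerPos, with location converted from the actor's local space to world space and rotation applied as stored, without the actor's transform.
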(event `self.ReceiveBeginPlay`
  (`|ExecutionSequence`
    (:`then_0`
      (`self.EnableInput` self (`GameplayStatics.GetPlayerController` 0)))
    (:`then_1`
      (`self.SetOwner` self (`GameplayStatics.GetPlayerController` 0)))))

(event `Key|T`
  (params (Key :type "Key Structure"))
  (bind (_playerpos_location _playerpos_rotation) (`KismetMathLibrary.BreakTransform` (`self.PlayerPos`)))
  ;[1 1 1] Add this actor in level and press T to teleport
  (:`Pressed`
    (bind _asbp_my_character (cast `/Game/Characters/My/BP_My_Character` (`GameplayStatics.GetPlayerCharacter` 0)))
    (`self.K2_SetActorLocationAndRotation` _asbp_my_character (`KismetMathLibrary.TransformLocation` (`self.GetTransform`) _playerpos_location) _playerpos_rotation false false)))

(fn `UserConstructionScript`)